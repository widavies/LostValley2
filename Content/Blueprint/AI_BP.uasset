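; AI character Blueprint that drives the running animation flag on its skeletal mesh.
; Each Tick it checks whether velocity is nonzero, casts the mesh's anim instance to PersonABP and sets CanRun to match.
; An unused movement-input check and a disconnected branch remain in the graph, and the construction script is empty.
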(event `self.ReceiveTick`
  (params (DeltaSeconds :type "Float (single-precision)"))
  (bind _returnvalue (`SkeletalMeshComponent.GetAnimInstance` (`self.Mesh`)))
  (if (not (== (`KismetMathLibrary.VSize` (`self.GetVelocity`)) 0.0))
    (bind _asperson_abp (cast `/Game/Blueprint/PersonABP` _returnvalue))
    (set `/Game/Blueprint/PersonABP.CanRun` true _asperson_abp)
    (else
      (bind _asperson_abp_2 (cast `/Game/Blueprint/PersonABP` _returnvalue))
      (set `/Game/Blueprint/PersonABP.CanRun` false _asperson_abp_2))))

(fn `UserConstructionScript`)